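; Gameplay ability for staff aiming that applies a camera modifier while the ability is active.
; An alternative-use pressed event adds an instance of the configured modifier class and stores it, while any other triggering event ends the ability immediately.
; Ending the ability removes the stored modifier.
; The camera manager is resolved through the owner actor's instigator controller and returned only for a local player controller.
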(event Ability|EventActivateAbilityFromEvent
  (params (EventData :type Gameplay%20Event%20Data%20Structure%20%28by%20ref%29))
  (if (== (.EventTag (Utilities|Struct|BreakGameplayEventData EventData)) "(TagName=\"Triggers.Actions.AlternativeUse.Pressed\")")
    (Camera|AddCameraModifier)
    (else
      (Ability|EndAbility))))

(event Ability|EventOnEndAbility
  (params (bWasCancelled :type Boolean))
  (Camera|RemoveCameraModifier))

(fn AddCameraModifier
  (bind _playercameramanager (Camera|GetCameraManager))
  (Utilities|IsValid _playercameramanager
    (:Is%20Valid
      (bind _returnvalue (Game|Player|AddNewCameraModifier _playercameramanager (Variables|Settings|GetCameraModifierClass)))
      (Variables|Internal|SetCameraModifier _returnvalue))))

(fn RemoveCameraModifier
  (bind _playercameramanager (Camera|GetCameraManager))
  (Utilities|IsValid _playercameramanager
    (:Is%20Valid
      (Game|Player|RemoveCameraModifier _playercameramanager (Variables|Internal|GetCameraModifier)))))

(fn GetCameraManager
  (bind _returnvalue (Ability|GetActorInfo))
  (bind _owneractor (Utilities|Struct|BreakGameplayAbilityActorInfo _returnvalue))
  (bind _returnvalue_2 (Game|GetInstigatorController _owneractor))
  (Utilities|IsValid _returnvalue_2
    (:Is%20Valid
      (bind _asplayer_controller (Utilities|Casting|CastToPlayerController _returnvalue_2))
      (if (Pawn|IsLocalPlayerController _asplayer_controller)
        (bind _playercameramanager (Variables|/Script/Engine.PlayerController|GetPlayerCameraManager _asplayer_controller)
          (:then
            (return _playercameramanager))
          (:else))))))