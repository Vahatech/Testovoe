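; Pickupable world item that grants gameplay abilities and a replicated gameplay tag to the actor that overlaps its box.
; Only the server accepts a pickup, and only if the item is unowned and the actor's Ability System Component lacks that tag.
; Pickup sets the owner, plays a montage on the actor and multicasts a Niagara burst.
; The Pickedup RepNotify attaches the mesh to the character's hand, disables collision and hides the idle effect.
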(event OnComponentBeginOverlap(Box)
  (params (OverlappedComponent :type Primitive%20Component%20Object%20Reference) (OtherActor :type Actor%20Object%20Reference) (OtherComp :type Primitive%20Component%20Object%20Reference) (OtherBodyIndex :type Integer) (bFromSweep :type Boolean) (SweepResult :type Hit%20Result%20Structure%20%28by%20ref%29))
  (if (OnPickup|CanPickup OtherActor)
    (OnPickup|HandlePickup OtherActor)
    (CallFunction|MulticastPlayPickupVFX)))

(event Custom|Multicast_PlayPickupVFX
  (Niagara|SpawnSystematLocation (Variables|OnPickup|GetPickupNiagara) (Transformation|GetActorLocation)))

(fn ConstructionScript)

(fn CanPickup
  (params (Interactor :type Actor%20Object%20Reference))
  (bind _returnvalue (Ability|GetAbilitySystemComponent Interactor))
  (Networking|SwitchHasAuthority
    (:Authority
      (Utilities|IsValid (Components|GetOwner)
        (:Is%20Not%20Valid
          (Utilities|IsValid _returnvalue
            (:Is%20Valid
              (bind _returnvalue_2 (GameplayTags|HasMatchingGameplayTag(Message) _returnvalue (Variables|OnPickup|GetGameplayTagToAdd)))
              (if (not _returnvalue_2)
                (return true)))))))))

(fn HandlePickup
  (params (Actor :type Actor%20Object%20Reference))
  (Actor|SetOwner Actor)
  (OnPickup|AddAbilitiestoOwner Actor)
  (OnPickup|AddTagtoOwner Actor)
  (Variables|Default|SetbPickedup true)
  (Class|BPRepliciatedAnimInterface|PlayMontage(Message) Actor (Variables|OnPickup|GetPickupMontage)))

(fn AddAbilitiestoOwner
  (params (Actor :type Actor%20Object%20Reference))
  (bind _returnvalue (Ability|GetAbilitySystemComponent Actor))
  (Utilities|IsValid _returnvalue
    (:Is%20Valid
      (for _array_element (Variables|OnPickup|GetAbilitiesToAdd)
        (GameplayAbilities|GiveAbility _returnvalue _array_element 0 -1))
      (return))))

(fn AddTagtoOwner
  (params (Actor :type Actor%20Object%20Reference))
  (Ability|GameplayEffect|AddLooseGameplayTags Actor (GameplayTags|MakeGameplayTagContainerfromTag (Variables|OnPickup|GetGameplayTagToAdd)) true))

(fn AttachItemtoOwner
  (bind _staticmesh (Variables|Default|GetStaticMesh))
  (bind _ascharacter (Utilities|Casting|CastToCharacter (Components|GetOwner)))
  (Transformation|AttachComponentToComponent _staticmesh (Variables|/Script/Engine.Character|GetMesh _ascharacter) "Hand_R" "KeepRelative" "KeepRelative" "KeepRelative" true)
  (Transformation|SetRelativeTransform _staticmesh (Variables|Default|GetAttachedRelativeTransform) false false))

(fn DisableItemCollision
  (Collision|SetCollisionEnabled (Variables|Default|GetStaticMesh) "NoCollision"))

(fn OnRepBPickedup
  (OnPickup|AttachItemtoOwner)
  (OnPickup|DisableItemCollision)
  (Rendering|SetVisibility (Variables|Default|GetNiagara) false false))