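; Base player character Blueprint that turns input into gameplay ability triggers and handles replicated montage playback.
; Enhanced Input primary and alternative actions send tagged gameplay events to the character itself, with separate pressed and released tags for the alternative action.
; PlayMontage runs only on the server and multicasts the montage, which is synchronously loaded and played on the character mesh.
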(event Custom|Multicast_PlayAnimMontage
  (params (InMontage :type Anim%20Montage%20Soft%20Object%20Reference))
  (bind _returnvalue (Utilities|LoadAssetBlocking InMontage))
  (Utilities|IsValid _returnvalue
    (:Is%20Valid
      (Animation|Montage|PlayMontage (Variables|Character|GetMesh) (Utilities|ResolveSoftReference InMontage)))))

(event EventPlayMontage
  (params (InMontage :type Anim%20Montage%20Soft%20Object%20Reference))
  (if (Networking|IsServer)
    (CallFunction|MulticastPlayAnimMontage InMontage)))

(event Input|EnhancedActionEvents|EnhancedInputActionIA_PrimaryAction
  (params (ActionValue :type Boolean) (ElapsedSeconds :type Float%20%28double-precision%29) (TriggeredSeconds :type Float%20%28double-precision%29) (InputAction :type Input%20Action%20Object%20Reference :default "/Game/Mechanics/Input/Actions/IA_PrimaryAction.IA_PrimaryAction"))
  ;[0.15 0.15 0.15 0.5] Used to activate gameplay abilities by "Gameplay Ability triggers"
  (Ability|SendGameplayEventtoActor self "(TagName=\"Triggers.Actions.PrimaryUse\")"))

(event Input|EnhancedActionEvents|EnhancedInputActionIA_AlternativeAction
  (params (ActionValue :type Boolean) (ElapsedSeconds :type Float%20%28double-precision%29) (TriggeredSeconds :type Float%20%28double-precision%29) (InputAction :type Input%20Action%20Object%20Reference :default "/Game/Mechanics/Input/Actions/IA_AlternativeAction.IA_AlternativeAction"))
  ;[0.15 0.15 0.15 0.5] Used to activate gameplay abilities by "Gameplay Ability triggers"
  (Ability|SendGameplayEventtoActor self (select ActionValue "(TagName=\"Triggers.Actions.AlternativeUse.Pressed\")" "(TagName=\"Triggers.Actions.AlternativeUse.Released\")")))

(fn ConstructionScript)